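; An in-world info text actor that displays the current game stage and a per-player scoreboard.
; On BeginPlay it binds to the state-changed event of BP_GS_GameState and writes each new stage's name to the stage text.
; For most stages it also rebuilds the score text from the GameState's patrol, coin, sneak, team and total score arrays.
; Player labels are generated from a fixed index range, not read from player data.
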(event Custom|StateChanged_Event
  (params (NewStage :type E_Stage%20Enum :default "NewEnumerator11"))
  (CallFunction|PrintStage NewStage)
  (switch Utilities|FlowControl|Switch|SwitchonE_Stage NewStage
    (:NewEnumerator11
      _)
    (:NewEnumerator19
      _)
    (:NewEnumerator23
      _)
    (:NewEnumerator27
      _)
    (:NewEnumerator28
      _))
  (CallFunction|AccessScore))

(event EventBeginPlay
  (bind _asbp_gs_game_state (Utilities|Casting|CastToBP_GS_GameState (Game|GetGameState)))
  (Variables|Default|SetState _asbp_gs_game_state)
  (EventDispatchers|AssignStateChanged _asbp_gs_game_state (delegate Custom|StateChanged_Event)))

(fn ConstructionScript)

(fn PrintStage
  (params (Stage :type E_Stage%20Enum :default "NewEnumerator11"))
  (Rendering|Components|TextRender|SetText (Variables|Default|GetTextInfo) (Utilities|Text|ToText(String) (Utilities|String|EnumtoString Stage))))

(fn PrintScore
  (params (Names :type Array%20of%20Strings) (PatrolScore :type Array%20of%20Integers) (CoinsScore :type Array%20of%20Integers) (SneakScore :type Array%20of%20Integers) (TeamScore :type Array%20of%20Integers) (Sums :type Array%20of%20Integers))
  (LocalVariables|SetScoreString "SCORE: <br>")
  (for (_array_element _array_index) Names
    (LocalVariables|SetScoreString (Utilities|String|Append (LocalVariables|GetScoreString) (Utilities|String|Append _array_element ": " (Utilities|String|ToString(Integer) (Utilities|Array|Get(acopy) PatrolScore _array_index)) "/" (Utilities|String|ToString(Integer) (Utilities|Array|Get(acopy) CoinsScore _array_index)) "/" (Utilities|String|ToString(Integer) (Utilities|Array|Get(acopy) SneakScore _array_index)) "/" (Utilities|String|ToString(Integer) (Utilities|Array|Get(acopy) TeamScore _array_index)) "/" (Utilities|String|ToString(Integer) (Utilities|Array|Get(acopy) Sums _array_index)) "<br>"))))
  (Rendering|Components|TextRender|SetText (Variables|Default|GetTextScore) (Utilities|Text|ToText(String) (LocalVariables|GetScoreString))))

(fn AccessScore
  (bind _state (Variables|Default|GetState))
  (for _index (range 0 5)
    (Utilities|Array|Add (LocalVariables|GetNames) (Utilities|String|BuildString(Integer) "Player" "_" _index)))
  (CallFunction|PrintScore (LocalVariables|GetNames) (Variables|/Game/GamePlay/Blueprints/BP_GS_GameState.BP_GS_GameState_C|GetPatrolScore _state) (Variables|/Game/GamePlay/Blueprints/BP_GS_GameState.BP_GS_GameState_C|GetCoinScore _state) (Variables|/Game/GamePlay/Blueprints/BP_GS_GameState.BP_GS_GameState_C|GetSneakScore _state) (Variables|/Game/GamePlay/Blueprints/BP_GS_GameState.BP_GS_GameState_C|GetTeamScore _state) (Variables|/Game/GamePlay/Blueprints/BP_GS_GameState.BP_GS_GameState_C|GetScore _state)))