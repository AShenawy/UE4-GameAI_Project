(event OnComponentBeginOverlap(Box)
  (params (OverlappedComponent :type Primitive%20Component%20Object%20Reference) (OtherActor :type Actor%20Object%20Reference) (OtherComp :type Primitive%20Component%20Object%20Reference) (OtherBodyIndex :type Integer) (bFromSweep :type Boolean) (SweepResult :type Hit%20Result%20Structure%20%28by%20ref%29))
  (switch Utilities|FlowControl|Switch|SwitchonE_Stage (Variables|/Game/GamePlay/Blueprints/BP_GS_GameState.BP_GS_GameState_C|GetStage (Variables|Default|GetState))
    (:NewEnumerator27
      (CallFunction|Visiting OtherActor false))))

(event OnComponentEndOverlap(Box)
  (params (OverlappedComponent :type Primitive%20Component%20Object%20Reference) (OtherActor :type Actor%20Object%20Reference) (OtherComp :type Primitive%20Component%20Object%20Reference) (OtherBodyIndex :type Integer))
  (switch Utilities|FlowControl|Switch|SwitchonE_Stage (Variables|/Game/GamePlay/Blueprints/BP_GS_GameState.BP_GS_GameState_C|GetStage (Variables|Default|GetState))
    (:NewEnumerator27
      (CallFunction|Visiting OtherActor true))))

(event Custom|StateChanged_Event_0
  (params (NewStage :type E_Stage%20Enum :default "NewEnumerator11"))
  (switch Utilities|FlowControl|Switch|SwitchonE_Stage NewStage
    (:NewEnumerator27
      (Rendering|SetVisibility (Variables|Default|GetTextRender) true false))))

(event EventBeginPlay
  (bind _asbp_gs_game_state (Utilities|Casting|CastToBP_GS_GameState (Game|GetGameState)))
  (bind _output_get (Variables|Default|SetState _asbp_gs_game_state))
  (EventDispatchers|AssignStateChanged _output_get (delegate Custom|StateChanged_Event_0)))

(fn ConstructionScript)

(fn Visiting
  (params (Actor :type Actor%20Object%20Reference) (IsLeaving :type Boolean))
  (bind _asai_character (Utilities|Casting|CastToAI_Character Actor))
  (Utilities|Array|SetArrayElem (Variables|Default|GetVisitedTeams) (Variables|/Game/GamePlay/Blueprints/AI_Character.AI_Character_C|GetTeamNr _asai_character) (+ (Utilities|Array|Get(acopy) (Variables|Default|GetVisitedTeams) (Variables|/Game/GamePlay/Blueprints/AI_Character.AI_Character_C|GetTeamNr _asai_character)) (Math|Integer|SelectInt -1 1 IsLeaving)))
  (if (== (Utilities|Array|Get(acopy) (Variables|Default|GetVisitedTeams) (Variables|/Game/GamePlay/Blueprints/AI_Character.AI_Character_C|GetTeamNr _asai_character)) 2)
    (bind _asbp_gs_game_state (Utilities|Casting|CastToBP_GS_GameState (Game|GetGameState)))
    (Default|SetTeamScore _asbp_gs_game_state (Variables|/Game/GamePlay/Blueprints/AI_Character.AI_Character_C|GetTeamNr _asai_character))))