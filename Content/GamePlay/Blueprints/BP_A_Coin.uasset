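; Coin actor that spins in place and bursts when an AI_Character overlaps it.
; BeginPlay picks a random spin direction and speed, which Tick applies as yaw to the Sphere component per frame, unscaled by delta time.
; Overlap by an AI_Character spawns an explosion particle and sound at the coin's location, then destroys it, with no score or count update here.
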(event EventBeginPlay
  (Variables|Default|SetRotationSpeed (* (Math|Integer|SelectInt 1 -1 (Math|Random|RandomBool)) (Math|Random|RandomFloatinRange 1.0 2.0))))

(event Collision|EventActorBeginOverlap
  (params (OtherActor :type Actor%20Object%20Reference))
  (bind _returnvalue (Transformation|GetActorLocation))
  (Utilities|Casting|CastToAI_Character OtherActor)
  (Effects|SpawnEmitteratLocation "/Game/GamePlay/Particles/P_Explosion.P_Explosion" _returnvalue)
  (Audio|SpawnSoundatLocation "/Game/GamePlay/Audio/Explosion_Cue.Explosion_Cue" _returnvalue "0, 0, 0" 0.5 1.0 0.0 0 0)
  (Actor|DestroyActor))

(event EventTick
  (params (DeltaSeconds :type Float%20%28single-precision%29))
  (Transformation|AddLocalRotation (Variables|Default|GetSphere) (Math|Rotator|MakeRotator 0.0 0.0 (Variables|Default|GetRotationSpeed)) false false))

(fn ConstructionScript)