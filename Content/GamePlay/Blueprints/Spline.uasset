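; Spline is a construction-time Blueprint that lays a configurable static mesh along a spline as a closed loop.
; The construction script adds one SplineMeshComponent per spline point, attached to the spline and deformed using that point's and the next point's local positions and tangents.
; The last segment wraps back to the first point, and each segment uses the chosen forward axis and query-only collision.
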(event EventBeginPlay)

(event Collision|EventActorBeginOverlap
  (params (OtherActor :type Actor%20Object%20Reference)))

(event EventTick
  (params (DeltaSeconds :type Float%20%28single-precision%29)))

(fn ConstructionScript
  (bind _spline (Variables|Default|GetSpline))
  (bind _output_get (LocalVariables|SetLastIndex (- (Spline|GetNumberOfSplinePoints (Variables|Default|GetSpline)) 1)))
  (for _index (range 0 _output_get)
    (LocalVariables|SetIndex _index)
    (bind _returnvalue (AddComponent|AddSplineMeshComponent false))
    (Components|StaticMesh|SetStaticMesh _returnvalue (Variables|Default|GetMesh))
    (SplineMesh|SetForwardAxis _returnvalue (Variables|Default|GetForward) true)
    (Transformation|AttachComponentToComponent _returnvalue (Variables|Default|GetSpline) "None" "KeepRelative" "KeepRelative" "KeepRelative" true)
    (SplineMesh|SetStartandEnd _returnvalue (Spline|GetLocationatSplinePoint _spline (LocalVariables|GetIndex) "Local") (Spline|GetTangentatSplinePoint _spline (LocalVariables|GetIndex) "Local") (Spline|GetLocationatSplinePoint _spline (select (== (LocalVariables|GetLastIndex) (LocalVariables|GetIndex)) 0 (+ (LocalVariables|GetIndex) 1)) "Local") (Spline|GetTangentatSplinePoint _spline (select (== (LocalVariables|GetLastIndex) (LocalVariables|GetIndex)) 0 (+ (LocalVariables|GetIndex) 1)) "Local") true :!class /Script/Engine.SplineMeshComponent)
    (Collision|SetCollisionEnabled _returnvalue "QueryOnly")))